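; Base AI creep for the MOBA spawn point system, a demo actor that reports its death to its spawner.
; Interface functions get and set its spawn point reference and in-spawn-area flag.
; On Destroyed, OnCreepHasDied calls CreepHasDied on the spawn point with authority only, printing a warning if the reference is invalid.
; Tick aligns the Name component to the first player controller's rotation, flipped 180 degrees.
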(event `self.ReceiveTick`
  (params (DeltaSeconds :type "Float (single-precision)"))
  (bind _name (`self.Name`))
  (bind (_returnvalue_location _returnvalue_rotation) (`KismetMathLibrary.BreakTransform` (`self.GetTransform` (`GameplayStatics.GetPlayerController` 0))))
  ;[0 0 0] Simple AI logic. Demo purposes only.
  (`SceneComponent.K2_SetWorldRotation` _name _returnvalue_rotation false false)
  (`SceneComponent.K2_AddLocalRotation` _name (struct :`Yaw` 180.0) false false))

(event `self.ReceiveBeginPlay`
  ;[0 0 0] Simple AI logic. Demo purposes only.
)

(event `self.ReceiveAnyDamage`
  (params (Damage :type "Float (single-precision)") (DamageType :type "DamageType Object Reference") (InstigatedBy :type "Controller Object Reference") (DamageCauser :type "Actor Object Reference"))
  ;[0 0 0] Simple AI logic. Demo purposes only.
)

(event `self.ReceiveDestroyed`
  ;[1 0 0] EVENT FOR WHEN THIS CREEP DIES, WE MUST CALL THE OnCreepHasDied INTERFACE EVENT SO THAT THE SPAWNER CAN UPDATE ITS INTERNAL VARIABLES.
  (`/Game/MOBASpawnPoints/Blueprints/ISpawnableCreep.OnCreepHasDied` (`self.SpawnPointReference`) self))

(fn `GetIsCreepInSpawnArea`
  (returns (bIsInSpawnArea :type Boolean))
  ;[0 0 0] Getter for the Spawn Area variable called through the Interface.
  (return (`self.bCreepIsInSpawnArea`)))

(fn `GetSpawnPoint`
  (returns (SpawnPoint :type "/Game/MOBASpawnPoints/Blueprints/BP_Base_SpawnPoint Object Reference"))
  ;[0 0 0] Getter for the Spawn Point reference called through the Interface.
  (return (`self.SpawnPointReference`)))

(fn `OnCreepHasDied`
  (params (SpawnPoint :type "/Game/MOBASpawnPoints/Blueprints/BP_Base_SpawnPoint Object Reference") (InCreep :type "Actor Object Reference"))
  (returns (OutCreep :type "Actor Object Reference"))
  ;[1 0 0] INTERFACE EVENT FOR WHEN THIS CREEP HAS DIED. THIS MUST BE CALLED WHEN THE CREEP DIES OR IS DESTROYED OTHERWISE THE SPAWNER WILL NOT RECIEVE THIS EVENT TO BE ABLE TO UPDATE INTERNAL VARIABLES.
  (`/Engine/EditorBlueprintResources/ActorMacros.Switch Has Authority`
    (:`Authority`
      (if (`KismetSystemLibrary.IsValid` SpawnPoint)
        (`/Game/MOBASpawnPoints/Blueprints/IMOBASpawner.CreepHasDied` SpawnPoint InCreep)
        (else
          (`KismetSystemLibrary.PrintString` "Warning: Creep cannot find where its SpawnPoint reference is." true true (struct :`R` 1.0 :`G` 1.0 :`A` 1.0)))))
    (:`Remote`
      _))
  (return InCreep))

(fn `SetIsCreepInSpawnArea`
  (params (IsInSpawnArea :type Boolean))
  (returns (bIsInSpawnArea :type Boolean))
  ;[0 0 0] Setter for the Spawn Area variable called through the Interface.
  (bind _output_get (set `self.bCreepIsInSpawnArea` IsInSpawnArea))
  (return _output_get))

(fn `SetSpawnPoint`
  (params (InSpawnPoint :type "/Game/MOBASpawnPoints/Blueprints/BP_Base_SpawnPoint Object Reference"))
  (returns (OutSpawnPoint :type "/Game/MOBASpawnPoints/Blueprints/BP_Base_SpawnPoint Object Reference"))
  ;[0 0 0] Setter for the Spawn Pointer reference called through the Interface.
  (bind _output_get (set `self.SpawnPointReference` InSpawnPoint))
  (return _output_get))

(fn `UserConstructionScript`)