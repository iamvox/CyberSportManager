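; Boss spawn point that spawns boss creeps on the server, first after an initial delay at BeginPlay.
; SpawnCreepWave spawns each class in CreepsToSpawn at the arrow's transform with a stagger delay, tracks it and passes itself via ISpawnableCreep.
; When RespawnBossOnlyWhenDead is set, spawning disables EnableTimer.
; CreepHasDied untracks the dead creep and re-enables that timer flag; no timer logic appears in this graph.
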(event `self.ReceiveBeginPlay`
  ;[0 0 0] Wait out the delay for the Boss to Spawn at the beginning of Play
  (`KismetSystemLibrary.Delay` (`self.InitialBossSpawnTimeInSeconds`))
  (`self.SpawnCreepWave`))

(event `/Game/MOBASpawnPoints/Blueprints/IMOBASpawner.SpawnCreepWave`
  ;[0 0 0] Determines if we can Spawn the Boss Creep and also sets up the Event Binding for the Respawn Timer.
  (`/Engine/EditorBlueprintResources/ActorMacros.Switch Has Authority`
    (:`Authority`
      (if (== (`KismetArrayLibrary.Array_Length` (`self.CreepsToSpawn`)) 0)
        (if (`self.bEnableDebugMessages`)
          (`KismetSystemLibrary.PrintString` "WARNING: No creeps to spawn from Boss Spawner!" true true (struct :`R` 1.0 :`G` 1.0 :`A` 1.0)))
        (else
          (if (`self.bRespawnBossOnlyWhenDead`)
            (set `self.bEnableTimer` false))
          (if (`self.bEnableDebugMessages`)
            (`KismetSystemLibrary.PrintString` "Spawning new Boss!"))
          (bind _array_element (`/Game/MOBASpawnPoints/Blueprints/BP_MOBA_MacroLibrary.ForEachLoopWithDelay` (`self.CreepsToSpawn`) :!label _label)
            (:`Loop Body`
              (bind _returnvalue (`|SpawnActorFromClass` _array_element (`SceneComponent.K2_GetComponentToWorld` (`self.ArrowForwardVector`)) "AdjustIfPossibleButAlwaysSpawn" "OverrideRootScale"))
              (`KismetArrayLibrary.Array_Add` (`self.SpawnedCreeps`) _returnvalue)
              ;;[1 0 0] THIS INTERFACE NEEDS TO BE IMPLEMENTED BY YOUR BASE AI CLASS TYPE
              (if (`KismetSystemLibrary.DoesImplementInterface` _returnvalue "/Game/MOBASpawnPoints/Blueprints/ISpawnableCreep.ISpawnableCreep_C")
                (message `/Game/MOBASpawnPoints/Blueprints/ISpawnableCreep.SetSpawnPoint` _returnvalue self)
                (elif (`self.bEnableDebugMessages`)
                  (`KismetSystemLibrary.PrintString` "WARNING: Spawned Actor does not implement the ISpawnableCreep interface from Boss Spawner!" true true (struct :`R` 1.0 :`G` 1.0 :`A` 1.0))))
              (`KismetSystemLibrary.Delay` (`self.PerCreepSpawnDelay`))
              (goto _label :!via `Next Iteration`))))))))

(event `/Game/MOBASpawnPoints/Blueprints/IMOBASpawner.CreepHasDied`
  (params (Creep :type "Actor Object Reference"))
  (bind _spawnedcreeps (`self.SpawnedCreeps`))
  ;[0 0 0] Event to notify this Spawner that the Boss Creep has died and to remove it from the Creeps list, as well as to enable the Spawn Timer.
  (for (_array_element _array_index) _spawnedcreeps
    (if (== _array_element Creep)
      (`KismetArrayLibrary.Array_Remove` _spawnedcreeps _array_index)
      (set `self.bEnableTimer` true)
      (break))))

(fn `UserConstructionScript`
  (`parent.UserConstructionScript`))