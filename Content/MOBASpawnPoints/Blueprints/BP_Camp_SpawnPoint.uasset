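; MOBA camp spawn point that spawns a group of creeps on the server, staggered by a delay, at per-creep offsets rotated by an arrow component.
; SpawnCreepWave requires all creeps dead, or only an empty camp when stack spawning is allowed.
; A trigger volume and death notifications track camp state through the ISpawnableCreep interface, with the last death re-enabling the timer flag.
; The construction script sizes the volume and adjusts the offset array toward the creep count.
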(event `self.ReceiveBeginPlay`
  ;[0 0 0] Enable our Spawn Timer to begin counting time when Play starts.
  (set `self.bEnableTimer` true))

(event `/Game/MOBASpawnPoints/Blueprints/IMOBASpawner.SpawnCreepWave`
  ;[0 0 0] Spawns each Camp Creep and also keeps track of how many Creeps are in the Spawn Area and if all Camp Creeps are Dead.
  (`/Engine/EditorBlueprintResources/ActorMacros.Switch Has Authority`
    (:`Authority`
      (if (== (`KismetArrayLibrary.Array_Length` (`self.CreepsToSpawn`)) 0)
        (if (`self.bEnableDebugMessages`)
          (`KismetSystemLibrary.PrintString` "WARNING: No creeps to spawn at Camp Spawner!" true true (struct :`R` 1.0 :`G` 1.0 :`A` 1.0)))
        (elif (`self.bAllowStackSpawning`)
          (if (`self.bIsCampEmpty`)
            (set `self.bIsCampEmpty` false :!label _label) ; We are Spawning Creeps so the camp is no longer Empty.
            (set `self.bAreAllCreepsDead` false)
            (if (`self.bEnableDebugMessages`)
              (`KismetSystemLibrary.PrintString` "Spawning new Camp Creeps!"))
            (bind (_array_element _array_index) (`/Game/MOBASpawnPoints/Blueprints/BP_MOBA_MacroLibrary.ForEachLoopWithDelay` (`self.CreepsToSpawn`) :!label _label_2)
              (:`Loop Body`
                (bind _returnvalue (`|SpawnActorFromClass` _array_element (`self.GetCreepSpawnLocation` _array_index (`self.CampCreepSpawnLocations`)) "AdjustIfPossibleButAlwaysSpawn" "OverrideRootScale"))
                (`KismetArrayLibrary.Array_Add` (`self.SpawnedCreeps`) _returnvalue)
                ;;[1 0 0] THIS INTERFACE NEEDS TO BE IMPLEMENTED BY YOUR BASE AI CLASS TYPE
                (if (`KismetSystemLibrary.DoesImplementInterface` _returnvalue "/Game/MOBASpawnPoints/Blueprints/ISpawnableCreep.ISpawnableCreep_C")
                  (message `/Game/MOBASpawnPoints/Blueprints/ISpawnableCreep.SetSpawnPoint` _returnvalue self)
                  (set `self.NumberOfCreepsInSpawnArea` (+ (`self.NumberOfCreepsInSpawnArea`) 1)) ; This creep has just spawned, so it must be within our Spawn Area.
                  (elif (`self.bEnableDebugMessages`)
                    (`KismetSystemLibrary.PrintString` "WARNING: Spawned Actor does not implement the ISpawnableCreep interface from Camp Spawner!" true true (struct :`R` 1.0 :`G` 1.0 :`A` 1.0))))
                (`KismetSystemLibrary.Delay` (`self.PerCreepSpawnDelay`))
                (goto _label_2 :!via `Next Iteration`))))
          (else
            (set `self.bEnableTimer` false)
            (if (`self.bAreAllCreepsDead`)
              (goto _label))))))))

(event `/Game/MOBASpawnPoints/Blueprints/IMOBASpawner.CreepHasDied`
  (params (Creep :type "Actor Object Reference"))
  (bind _spawnedcreeps (`self.SpawnedCreeps`))
  ;[0 0 0] Event to notify the Spawner that a Camp Creep has died and to update a few variables as well as remove it from the internal array of Creeps.
  (for (_array_element _array_index) _spawnedcreeps
    (if (== _array_element Creep)
      (`KismetArrayLibrary.Array_Remove` _spawnedcreeps _array_index)
      (break)))
  (if (== (`KismetArrayLibrary.Array_Length` _spawnedcreeps) 0)
    (set `self.bIsCampEmpty` true)
    (set `self.bAreAllCreepsDead` true)
    (set `self.bEnableTimer` true) ; All Creeps are now dead, so we need to Enable the Spawn Timer to start again.
  ))

(event `self.SpawnAreaTriggerVolume.OnComponentBeginOverlap`
  (params (OtherActor :type "Actor Object Reference") (OtherComp :type "PrimitiveComponent Object Reference") (OtherBodyIndex :type Integer) (bFromSweep :type Boolean) (SweepResult :type "HitResult Structure (by ref)"))
  ;[0 0 0] Spawn Area collision detection, determines if the Camp is empty or not and updates incoming and outgoing Creeps status variables to reflect these changes.
  ;;[1 0 0] THIS INTERFACE NEEDS TO BE IMPLEMENTED BY YOUR BASE AI CLASS TYPE
  (if (`KismetSystemLibrary.DoesImplementInterface` OtherActor "/Game/MOBASpawnPoints/Blueprints/ISpawnableCreep.ISpawnableCreep_C")
    ;;[0 1 0] If the Actor came from this Camp, then the Camp is not empty and we need to reflect this change.
    (for _array_element (`self.SpawnedCreeps`)
      (if (== _array_element OtherActor)
        (message `/Game/MOBASpawnPoints/Blueprints/ISpawnableCreep.SetIsCreepInSpawnArea` OtherActor true)
        (set `self.bIsCampEmpty` false)
        (break)))))

(event `self.SpawnAreaTriggerVolume.OnComponentEndOverlap`
  (params (OtherActor :type "Actor Object Reference") (OtherComp :type "PrimitiveComponent Object Reference") (OtherBodyIndex :type Integer))
  ;[0 0 0] Spawn Area collision detection, determines if the Camp is empty or not and updates incoming and outgoing Creeps status variables to reflect these changes.
  ;;[1 0 0] THIS INTERFACE NEEDS TO BE IMPLEMENTED BY YOUR BASE AI CLASS TYPE
  (if (`KismetSystemLibrary.DoesImplementInterface` OtherActor "/Game/MOBASpawnPoints/Blueprints/ISpawnableCreep.ISpawnableCreep_C")
    ;;[0 1 0] If the Actor leaving the volume is any of our Camp Creeps, then we need to do a check to see if it was the last Camp Creep to leave the volume.
    (for _array_element (`self.SpawnedCreeps`)
      (bind _bisinspawnarea (message `/Game/MOBASpawnPoints/Blueprints/ISpawnableCreep.GetIsCreepInSpawnArea` OtherActor))
      (if (and _bisinspawnarea (== _array_element OtherActor))
        (message `/Game/MOBASpawnPoints/Blueprints/ISpawnableCreep.SetIsCreepInSpawnArea` OtherActor false)
        (set `self.NumberOfCreepsInSpawnArea` (- (`self.NumberOfCreepsInSpawnArea`) 1))
        (break)))
    (if (== (`self.NumberOfCreepsInSpawnArea`) 0)
      (set `self.bIsCampEmpty` true))))

(fn `GetCreepSpawnLocation`
  (params (Index :type Integer) (Creeps :type "Array of Vector Structure"))
  (returns (Location :type "Transform Structure"))
  (bind _arrowforwardvector (`self.ArrowForwardVector`))
  (bind _returnvalue (`SceneComponent.K2_GetComponentRotation` _arrowforwardvector))
  ;[0 0 0] Get the individual spawn locations matched to the Creeps order of appearance.
  (return (`KismetMathLibrary.MakeTransform` (+ (`KismetMathLibrary.GreaterGreater_VectorRotator` (`KismetArrayLibrary.Array_Get` Creeps Index) _returnvalue) (`SceneComponent.K2_GetComponentLocation` _arrowforwardvector)) _returnvalue)))

(fn `UserConstructionScript`
  (bind (_spawnareatransform_location _spawnareatransform_rotation _spawnareatransform_scale) (`KismetMathLibrary.BreakTransform` (`self.SpawnAreaTransform`)))
  (bind _spawnareatriggervolume (`self.SpawnAreaTriggerVolume`))
  (bind _campcreepspawnlocations (`self.CampCreepSpawnLocations`))
  (bind _returnvalue (`KismetArrayLibrary.Array_Length` (`self.CreepsToSpawn`)))
  (bind _returnvalue_2 (`KismetArrayLibrary.Array_Length` _campcreepspawnlocations))
  ;[0 0 0] Setup the trigger volume and offset Vectors
  (`parent.UserConstructionScript`)
  (`SceneComponent.K2_SetRelativeTransform` _spawnareatriggervolume (`KismetMathLibrary.MakeTransform` _spawnareatransform_location _spawnareatransform_rotation) false false)
  (`BoxComponent.SetBoxExtent` _spawnareatriggervolume _spawnareatransform_scale true) ; Instead of altering the Scale of the TriggerVolume, we need to scale its Extents.
  ;;[0 1 0] Build the Array of Vectors to allow offsetting the position of each Camp Creep.
  (if (> _returnvalue 0)
    (for _ (range _returnvalue)
      (if (== _returnvalue _returnvalue_2)
        _
        (elif (< _returnvalue _returnvalue_2)
          (`KismetArrayLibrary.Array_Remove` _campcreepspawnlocations)
          (elif (> _returnvalue _returnvalue_2)
            (`KismetArrayLibrary.Array_Add` _campcreepspawnlocations (0.0 0.0 0.0))
            (else
              (`KismetArrayLibrary.Array_Clear` _campcreepspawnlocations))))))))