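; Test Actor Blueprint that prototypes random character generation from the NamesListCSV data table.
; On BeginPlay it looks up one random row by converting a small random integer into a row name, but does nothing with the result.
; Disconnected nodes would set Name and Surname from separate random rows and roll Potential between Skill and a fixed cap, but they never run.
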(event `self.ReceiveBeginPlay`
  (bind _returnvalue (`|GetDataTableRow` "/Game/DatabasesStuff/OldStuff/NamesListCSV.NamesListCSV" (`KismetStringLibrary.Conv_StringToName` (`KismetStringLibrary.Concat_StrStr` (`KismetStringLibrary.Conv_IntToString` (`KismetMathLibrary.RandomInteger` 5)))))))

(fn `UserConstructionScript`)