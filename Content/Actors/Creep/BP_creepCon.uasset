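; AI controller for melee creeps that runs their behavior tree and starts them at their first waypoint.
; A looping timer polls sight perception, collects living characters of other teams via interface messages, and prunes invalid or dead ones.
; It writes the enemy and creep state to the blackboard.
; An event dispatcher fired each tick triggers the check that returns the creep to waypoint movement when no valid first enemy remains.
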(event `self.OnPossess`
  (params (PossessedPawn :type "Pawn Object Reference"))
  (bind _returnvalue (`AIBlueprintHelperLibrary.GetBlackboard` null))
  (`self.RunBehaviorTree` "/Game/Actors/Creep/BP_CreepBT.BP_CreepBT")
  (bind _asmelee_creep (cast `/Game/Actors/Creep/meleeCreep` PossessedPawn)
    (:`then`
      ;[0.8879 0.235 1] Setting blackboard values
      (`BlackboardComponent.SetValueAsInt` _returnvalue (`self.CurrentWaypointKey`) 0)
      (`BlackboardComponent.SetValueAsObject` _returnvalue (`self.TargetActorKey`) (`KismetArrayLibrary.Array_Get` (`/Game/Actors/Creep/meleeCreep.Waypoints` _asmelee_creep)))
      (`KismetSystemLibrary.K2_SetTimerDelegate` (delegate `TickEveryX`) (`self.TickTime`) true))
    (:`CastFailed`
      (`KismetSystemLibrary.PrintString` "Cast to creep failed. WHAT DID U D0?"))))

(event `TickEveryX`
  (bind _returnvalue (`AIBlueprintHelperLibrary.GetBlackboard` null))
  (bind _enemies (`self.Enemies`))
  ;[0.06089 1 0] Checks If Actor is an Enemy and places it into array if it is
  (`self.Dispatch_TickEveryX`)
  (add `self.Dispatch_TickEveryX` (delegate `IsThereEnemies?`))
  (for _array_element (`AIPerceptionComponent.GetCurrentlyPerceivedActors` (`self.AIPerception`) "/Script/AIModule.AISense_Sight")
    (if (`KismetSystemLibrary.DoesImplementInterface` _array_element "/Game/Actors/Interfaces/BPI_GenericCharOnMap.BPI_GenericCharOnMap_C")
      (bind _team (message `/Game/Actors/Interfaces/BPI_GenericCharOnMap.Get_Team` _array_element))
      (if (not (== _team (`/Game/Actors/Creep/meleeCreep.Team` (stale `self.OnPossess` _asmelee_creep))))
        (`KismetArrayLibrary.Array_AddUnique` _enemies _array_element)
        (for (_array_element_2 _array_index) _enemies
          (if (`KismetSystemLibrary.IsValid` _array_element_2)
            (bind _isalive (message `/Game/Actors/Interfaces/BPI_GenericCharOnMap.Get_IsAlive` _array_element_2))
            (if _isalive
              ;[1 0 0] Set Enemy Key
              (`BlackboardComponent.SetValueAsObject` _returnvalue (`self.EnemyKey`) _array_element_2)
              ;[1 0 0] Set Creep State
              (`BlackboardComponent.SetValueAsEnum` _returnvalue (`self.CreepStateKey`) (enumliteral `/Game/Actors/Creep/CreepState` "NewEnumerator0"))
              (else
                (`KismetArrayLibrary.Array_Remove` _enemies _array_index :!label _label)))
            (else
              (goto _label))))))))

(event `IsThereEnemies?`
  (if (not (`KismetSystemLibrary.IsValid` (`KismetArrayLibrary.Array_Get` (`self.Enemies`))))
    ;[0 1 0] Set State to Move to Waypoint
    (`BlackboardComponent.SetValueAsEnum` (`AIBlueprintHelperLibrary.GetBlackboard` null) (`self.CreepStateKey`) (enumliteral `/Game/Actors/Creep/CreepState` "NewEnumerator1"))))

(fn `UserConstructionScript`)