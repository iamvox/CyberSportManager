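; Game mode that builds the lane waypoint paths for Radiant and Dire creeps in a three-lane MOBA setup.
; On BeginPlay it gathers all WaypointTest actors and slots each into a Radiant array by its Lane and Index.
; The Dire arrays are reversed copies of those, made by inserting each waypoint at the front.
; GetWaypoints returns one of the six team-lane arrays by index.
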(event `self.ReceiveBeginPlay`
  (bind _team0lane0 (`self.team0Lane0`))
  (bind _team0lane1 (`self.team0Lane1`))
  (bind _team0lane2 (`self.team0Lane2`))
  (bind _outactors (`GameplayStatics.GetAllActorsOfClass` "/Game/Actors/Creep/WaypointTest.WaypointTest_C"))
  ;[1 1 1] Lane arrays for radiant creeps
  (for _array_element _outactors
    (switch `int` (`/Game/Actors/Creep/WaypointTest.Lane` _array_element)
      (:`0`
        (bind _index (`/Game/Actors/Creep/WaypointTest.index` _array_element))
        (`KismetArrayLibrary.Array_Set` _team0lane0 _index _array_element))
      (:`1`
        (`KismetArrayLibrary.Array_Set` _team0lane1 _index _array_element))
      (:`2`
        (`KismetArrayLibrary.Array_Set` _team0lane2 _index _array_element))))
  ;[1 1 1] Lane arrays for dire creeps
  (for _array_element_2 _team0lane0
    (`KismetArrayLibrary.Array_Insert` (`self.team1Lane0`) _array_element_2))
  (for _array_element_3 _team0lane1
    (`KismetArrayLibrary.Array_Insert` (`self.team1Lane1`) _array_element_3))
  (for _array_element_4 _team0lane2
    (`KismetArrayLibrary.Array_Insert` (`self.team1Lane2`) _array_element_4)))

(fn `getWaypoints`
  (params (Index :type Integer))
  (returns (Waypoints :type "Array of /Game/Actors/Creep/WaypointTest Object Reference"))
  (return (select `int` Index :`0` (`self.team0Lane0`) :`1` (`self.team0Lane1`) :`2` (`self.team0Lane2`) :`3` (`self.team1Lane0`) :`4` (`self.team1Lane1`) :`5` (`self.team1Lane2`))))

(fn `UserConstructionScript`)