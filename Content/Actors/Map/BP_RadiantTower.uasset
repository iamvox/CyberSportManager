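; BP_RadiantTower is a map tower that damages characters on other teams that it sees.
; A looping timer polls AI Perception sight for BPI_GenericCharOnMap actors, adding those with a different team to an Enemies list.
; Each such sighting iterates that list, removing invalid or dead entries and calling Attck to apply damage after a Delay placed inside the loop.
; Its stat and team getters and setters are stubs returning default values.
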(event `self.ReceiveBeginPlay`
  ;[0 0 0] TickEveryN
  (`KismetSystemLibrary.K2_SetTimerDelegate` (delegate `TickEveryX`) (`self.TickTime`) true))

(event `TickEveryX`
  (bind _enemies (`self.Enemies`))
  ;[0 0 0] TickEveryN
  (for _array_element (`AIPerceptionComponent.GetCurrentlyPerceivedActors` (`self.AIPerception`) "/Script/AIModule.AISense_Sight")
    (if (`KismetSystemLibrary.DoesImplementInterface` _array_element "/Game/Actors/Interfaces/BPI_GenericCharOnMap.BPI_GenericCharOnMap_C")
      (bind _team (message `/Game/Actors/Interfaces/BPI_GenericCharOnMap.Get_Team` _array_element))
      (if (not (== _team (`self.Team`)))
        (`KismetArrayLibrary.Array_AddUnique` _enemies _array_element)
        (for (_array_element_2 _array_index) _enemies
          (if (`KismetSystemLibrary.IsValid` _array_element_2)
            (bind _isalive (message `/Game/Actors/Interfaces/BPI_GenericCharOnMap.Get_IsAlive` _array_element_2))
            (if _isalive
              (`KismetSystemLibrary.Delay` 1.0)
              (`self.Attck` _array_element_2)
              (else
                (`KismetArrayLibrary.Array_RemoveItem` _enemies _array_element_2)))
            (else
              (`KismetArrayLibrary.Array_Remove` _enemies _array_index))))))))

(fn `Attck`
  (params (Enemy :type "Actor Object Reference"))
  (returns (IsSucceded :type Boolean))
  (`GameplayStatics.ApplyDamage` Enemy (`self.Damage`) null self)
  (return false))

(fn `Get_AttackSpeed`
  (returns (`Attack Speed` :type "Float (double-precision)"))
  (return 0.0))

(fn `Get_Damage`
  (returns (damage :type "Float (double-precision)"))
  (return 0.0))

(fn `Get_Health`
  (returns (Health :type "Float (double-precision)"))
  (return 0.0))

(fn `Get_IsAlive`
  (returns (IsAlive :type Boolean))
  (return false))

(fn `Get_Team`
  (returns (Team :type Integer))
  (return 0))

(fn `Set_Health`
  (params (Health :type "Float (double-precision)"))
  (returns (`Updated Health` :type "Float (double-precision)"))
  (return 0.0))

(fn `Set_IsAlive`
  (params (IsAlive :type Boolean))
  (returns (IsAliveUpdated :type Boolean))
  (return false))

(fn `UserConstructionScript`)