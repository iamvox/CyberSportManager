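; Team-based map tower that spots opposing characters by sight, attacks them, and destroys itself when its health runs out.
; A looping timer polls AI Perception, filters actors through BPI_GenericCharOnMap by team, and adds them to an Enemies list.
; Each opposing sighting rescans that list, pruning dead or invalid entries and applying damage after a one-second Delay inside the loop, so attacks do not queue per enemy.
; BeginPlay also passes the team to BPFOWHideComponent.
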(event `self.ReceiveBeginPlay`
  (set `/Game/ClassicRTSFOW/Blueprints/BP_FOW_HideComponent.Team` (`self.Team`) (`self.BP_FOW_HideComponent`))
  ;[0 0 0] TickEveryN
  (`KismetSystemLibrary.K2_SetTimerDelegate` (delegate `TickEveryX`) (`self.TickTime`) true))

(event `TickEveryX`
  (bind _enemies (`self.Enemies`))
  ;[0 0 0] TickEveryN
  (for _array_element (`AIPerceptionComponent.GetCurrentlyPerceivedActors` (`self.AIPerception`) "/Script/AIModule.AISense_Sight")
    (if (`KismetSystemLibrary.DoesImplementInterface` _array_element "/Game/Actors/Interfaces/BPI_GenericCharOnMap.BPI_GenericCharOnMap_C")
      (bind _team (message `/Game/Actors/Interfaces/BPI_GenericCharOnMap.Get_Team` _array_element))
      (if (not (== _team (`self.Team`)))
        (`KismetArrayLibrary.Array_AddUnique` _enemies _array_element)
        (for (_array_element_2 _array_index) _enemies
          (if (`KismetSystemLibrary.IsValid` _array_element_2)
            (bind _isalive (message `/Game/Actors/Interfaces/BPI_GenericCharOnMap.Get_IsAlive` _array_element_2))
            (if _isalive
              (`KismetSystemLibrary.Delay` 1.0)
              (`self.Attack` _array_element_2)
              (else
                (`KismetArrayLibrary.Array_RemoveItem` _enemies _array_element_2)))
            (else
              (`KismetArrayLibrary.Array_Remove` _enemies _array_index))))))))

(event `self.ReceiveAnyDamage`
  (params (Damage :type "Float (single-precision)") (DamageType :type "DamageType Object Reference") (InstigatedBy :type "Controller Object Reference") (DamageCauser :type "Actor Object Reference"))
  ;[0 0 0] Applies damage, checks if IsAlive
  (bind _output_get (set `self.Health` (- (`self.Health`) Damage)))
  (if (> _output_get 0.0)
    (set `self.Is Alive` true)
    (else
      (set `self.Is Alive` false)
      (`self.K2_DestroyActor` self))))

(fn `Attack`
  (params (Enemy :type "Actor Object Reference"))
  (returns (`Is Succeeded` :type Boolean))
  (`GameplayStatics.ApplyDamage` Enemy (`self.Damage`) null self)
  (return true))

(fn `Get_AttackSpeed`
  (returns (`Attack Speed` :type "Float (double-precision)"))
  (return 0.0))

(fn `Get_Damage`
  (returns (damage :type "Float (double-precision)"))
  (return (`self.Damage`)))

(fn `Get_Health`
  (returns (Health :type "Float (double-precision)"))
  (return (`self.Health`)))

(fn `Get_IsAlive`
  (returns (IsAlive :type Boolean))
  (return (`self.Is Alive`)))

(fn `Get_Team`
  (returns (Team :type Integer))
  (return (`self.Team`)))

(fn `Set_Health`
  (params (Health :type "Float (double-precision)"))
  (returns (`Updated Health` :type "Float (double-precision)"))
  (bind _output_get (set `self.Health` Health))
  (return _output_get))

(fn `Set_IsAlive`
  (params (IsAlive :type Boolean))
  (returns (IsAliveUpdated :type Boolean))
  (bind _output_get (set `self.Is Alive` IsAlive))
  (return _output_get))

(fn `UserConstructionScript`)