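; BP_RadiantAncient is a map actor for the Radiant Ancient, currently a skeleton with no gameplay behavior.
; Its event graph holds only disabled default events, and its construction script is empty.
; Getters and setters for combat stats, team and alive state are stubs that return zero or false, and the setters store nothing.
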(fn `Get_AttackSpeed`
  (returns (`Attack Speed` :type "Float (double-precision)"))
  (return 0.0))

(fn `Get_Damage`
  (returns (damage :type "Float (double-precision)"))
  (return 0.0))

(fn `Get_Health`
  (returns (Health :type "Float (double-precision)"))
  (return 0.0))

(fn `Get_IsAlive`
  (returns (IsAlive :type Boolean))
  (return false))

(fn `Get_Team`
  (returns (Team :type Integer))
  (return 0))

(fn `Set_Health`
  (params (Health :type "Float (double-precision)"))
  (returns (`Updated Health` :type "Float (double-precision)"))
  (return 0.0))

(fn `Set_IsAlive`
  (params (IsAlive :type Boolean))
  (returns (IsAliveUpdated :type Boolean))
  (return false))

(fn `UserConstructionScript`)