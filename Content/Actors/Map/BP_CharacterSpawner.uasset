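; BP_CharacterSpawner is a map actor that spawns a batch of MainCharacter actors for its team when play begins.
; Each spawns at a random reachable navigation point around the spawner, with collision adjustment so spawning always succeeds, and inherits the spawner's Team.
; It also exposes team and combat-stat accessors, of which only the Team getter returns real data while health, damage, attack speed and alive-state functions are stubs.
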(event `self.ReceiveBeginPlay`
  (bind _returnvalue_location (`KismetMathLibrary.BreakTransform` (`self.GetTransform` self)))
  (for _ (range 5)
    (bind _returnvalue (`|SpawnActorFromClass` "/Game/Actors/Character/AI/mainCharacter.mainCharacter_C" (`KismetMathLibrary.MakeTransform` (`NavigationSystem.GetRandomReachablePointInRadius` _returnvalue_location 700.0)) "AdjustIfPossibleButAlwaysSpawn" "OverrideRootScale"))
    (set `/Game/Actors/Character/AI/mainCharacter.Team` (`self.Team`) _returnvalue)))

(fn `Get_AttackSpeed`
  (returns (`Attack Speed` :type "Float (double-precision)"))
  (return 0.0))

(fn `Get_Damage`
  (returns (damage :type "Float (double-precision)"))
  (return 0.0))

(fn `Get_Health`
  (returns (Health :type "Float (double-precision)"))
  (return 0.0))

(fn `Get_IsAlive`
  (returns (IsAlive :type Boolean))
  (return false))

(fn `Get_Team`
  (returns (Team :type Integer))
  (return (`self.Team`)))

(fn `Set_Health`
  (params (Health :type "Float (double-precision)"))
  (returns (`Updated Health` :type "Float (double-precision)"))
  (return 0.0))

(fn `Set_IsAlive`
  (params (IsAlive :type Boolean))
  (returns (IsAliveUpdated :type Boolean))
  (return false))

(fn `UserConstructionScript`)