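; BP_HeightmapTile is a placeable cube that marks a height level on the fog-of-war tile grid.
; Its construction script reads tile settings from the first BP_FOW_Actor, snapping position and scale to whole tiles, with half-tile offsets for odd sizes.
; Height comes from the actor's Z scale and tints a dynamic material from green toward red.
; The FOW actor's ShowHeightmap flag toggles the cube's visibility.
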(fn `UserConstructionScript`
  (locals (FOW_Actor :type "/Game/ClassicRTSFOW/Blueprints/BP_FOW_Actor Object Reference"))
  (bind (_returnvalue_x _returnvalue_y) (`KismetMathLibrary.BreakVector` (`self.K2_GetActorLocation`)))
  (bind (_returnvalue_x_2 _returnvalue_y_2) (`KismetMathLibrary.BreakVector` (`self.GetActorScale3D`)))
  (bind (_returnvalue_x_3 _returnvalue_y_3 _returnvalue_z) (`KismetMathLibrary.BreakVector` (`self.GetActorScale3D`)))
  (bind _returnvalue_x_4 (`KismetMathLibrary.BreakVector` (`self.GetActorScale3D`)))
  (bind _fow_actor (`local.FOW_Actor`))
  (bind _returnvalue (/ (`self.Tilesize`) 100.0))
  (bind _returnvalue_2 (`KismetMathLibrary.FTrunc` _returnvalue_z))
  (bind _returnvalue_3 (/ (`KismetMathLibrary.Conv_IntToDouble` (`self.Height`)) 4.0))
  (bind _returnvalue_4 (* (`KismetMathLibrary.Conv_IntToDouble` (`.ReturnValue` (`KismetMathLibrary.FMod` _returnvalue_x (`self.Tilesize`)))) (`self.Tilesize`)))
  (bind _returnvalue_5 (* (`KismetMathLibrary.Conv_IntToDouble` (`.ReturnValue` (`KismetMathLibrary.FMod` _returnvalue_y (`self.Tilesize`)))) (`self.Tilesize`)))
  (bind _outactors (`GameplayStatics.GetAllActorsOfClass` "/Game/ClassicRTSFOW/Blueprints/BP_FOW_Actor.BP_FOW_Actor_C"))
  (bind _output_get (set `local.FOW_Actor` (`KismetArrayLibrary.Array_Get` _outactors)))
  (set `self.Tilesize` (`/Game/ClassicRTSFOW/Blueprints/BP_FOW_Actor.Tilesize` _output_get))
  (`|ExecutionSequence`
    (:`then_0`
      ;[0.4805 0 0.825] Snap the location of this actor to the WorldGrid
      (`SceneComponent.K2_SetWorldLocation` (`self.Cube`) (`KismetMathLibrary.MakeVector` (select `int` (mod (`KismetMathLibrary.FTrunc` _returnvalue_x_4) 2) :`0` _returnvalue_4 :`1` (+ _returnvalue_4 (* (`self.Tilesize`) 0.5))) (select `int` (mod (`KismetMathLibrary.FTrunc` _returnvalue_y_2) 2) :`0` _returnvalue_5 :`1` (+ _returnvalue_5 (* (`self.Tilesize`) 0.5))) (- (+ (`/Game/ClassicRTSFOW/Blueprints/BP_FOW_Actor.ZPosition` _fow_actor) (* (* (`/Game/ClassicRTSFOW/Blueprints/BP_FOW_Actor.ZScalePerTile` _fow_actor) 100.0) (`KismetMathLibrary.Conv_IntToDouble` (`self.Height`)) 0.5)) 25.0)) false false))
    (:`then_1`
      ;[0.4805 0 0.825] Snap the scale of this actor to a fixed number of WorldGrid tiles
      (`SceneComponent.SetWorldScale3D` (`self.Cube`) (`KismetMathLibrary.MakeVector` (* (`KismetMathLibrary.Conv_IntToDouble` (`KismetMathLibrary.FTrunc` _returnvalue_x_3)) _returnvalue) (* _returnvalue (`KismetMathLibrary.Conv_IntToDouble` (`KismetMathLibrary.FTrunc` _returnvalue_y_3))) (* (`KismetMathLibrary.Conv_IntToDouble` _returnvalue_2) (`/Game/ClassicRTSFOW/Blueprints/BP_FOW_Actor.ZScalePerTile` (`local.FOW_Actor`)))))
      (set `self.Height` _returnvalue_2))
    (:`then_2`
      ;[0.4805 0 0.825] Set the color of this actor depending on its height
      (bind _returnvalue_6 (`PrimitiveComponent.CreateDynamicMaterialInstance` (`self.Cube`) 0 "/Game/ClassicRTSFOW/Materials/Mat_HeightmapColor.Mat_HeightmapColor"))
      (`MaterialInstanceDynamic.SetVectorParameterValue` _returnvalue_6 "Color" (make `LinearColor` _returnvalue_3 (- 1.0 _returnvalue_3))))
    (:`then_3`
      (if (`/Game/ClassicRTSFOW/Blueprints/BP_FOW_Actor.ShowHeightmap` (`local.FOW_Actor`))
        (`SceneComponent.SetHiddenInGame` (`self.DefaultSceneRoot`) false true)
        (`SceneComponent.SetVisibility` (`self.Cube`) true true)
        (else
          (`SceneComponent.SetHiddenInGame` (`self.DefaultSceneRoot`) true true)
          (`SceneComponent.SetVisibility` (`self.Cube`) false true))))))