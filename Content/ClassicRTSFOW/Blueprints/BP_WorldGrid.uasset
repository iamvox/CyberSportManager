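; World grid for an RTS fog of war, tracking discovered and visible state plus terrain height per tile in flattened 1D arrays.
; Discover walks precomputed lines from each unit, stopping at higher terrain for line of sight, marking tiles by fade time or static-viewer lists.
; Height edits force affected static vision components to reload.
; A loaded view window is kept as per-row start and end indices, making moves cheap.
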(fn `ChangeHeightmapTile`
  (params (Location :type "Vector2D Structure") (NewHeight :type Integer))
  (locals (NewHeightL :type Integer) (NTilesL :type Integer :default 0) (X0L :type Integer) (Y0L :type Integer) (XL :type Integer) (YL :type Integer) (Components :type "Array of /Game/ClassicRTSFOW/Blueprints/BP_FOW_VisionComponent Object Reference") (CurrentComponent :type "/Game/ClassicRTSFOW/Blueprints/BP_FOW_VisionComponent Object Reference"))
  (bind _visionrange (`/Game/ClassicRTSFOW/Blueprints/BP_FOW_VisionComponent.VisionRange` (`local.CurrentComponent`)))
  (bind (_item_discovered _item_fadetime _item_visiblebystatic) (break `/Game/ClassicRTSFOW/Blueprints/Structs/BP_Tile` (`KismetArrayLibrary.Array_Get` (`self.Grid`) (`self.Get1DGridIndex` (`local.XL`) (`local.YL`)))))
  ;[0.4805 0 0.825] Change the height of the tile at Location to the desired value
  (set `local.NewHeightL` NewHeight)
  (bind (_x _y) (`self.TransformWorldToGridLocation` Location))
  (set `local.X0L` _x)
  (set `local.Y0L` _y)
  (`KismetArrayLibrary.Array_Set` (`self.Heightmap`) (`self.Get1DGridIndex` (`local.X0L`) (`local.Y0L`)) (`local.NewHeightL`))
  (`|ExecutionSequence`
    (:`then_0`
      ;[0.0412 0.655 0.4066] Loop over all tiles within the (squared) maximum vision range to find out if there are vision actors with static vision that needs to be updated
      (set `local.NTilesL` (`KismetMathLibrary.FTrunc` (/ (`self.MaxVisionRange`) (`self.Tilesize`))))
      (for _index (range (- (`local.X0L`) (`local.NTilesL`)) (+ (+ (`local.X0L`) (`local.NTilesL`)) 1))
        (set `local.XL` _index)
        (for _index_2 (range (- (`local.Y0L`) (`local.NTilesL`)) (+ (+ (`local.Y0L`) (`local.NTilesL`)) 1))
          (set `local.YL` _index_2)
          ;[0.2236 0.505 0.07345] Find all vision actor components with currently static vision within the (squared) maximum vision range of the changed HeightmapTile.
          (for _array_element _item_visiblebystatic
            (if (`/Game/ClassicRTSFOW/Blueprints/BP_FOW_VisionComponent.GetStatic` _array_element)
              (`KismetArrayLibrary.Array_AddUnique` (`local.Components`) _array_element))))))
    (:`then_1`
      ;[0.0412 0.655 0.4066] Loop over all components whose actors are in maximum vision range of the changed HeightmapTIle
      (for _array_element_2 (`local.Components`)
        (bind _output_get (set `local.CurrentComponent` _array_element_2))
        (bind (_returnvalue_x _returnvalue_y) (`KismetMathLibrary.BreakVector` (`Actor.K2_GetActorLocation` (`ActorComponent.GetOwner` _output_get))))
        ;[0.54 0.04036 0] Check if the changed HeightmapTile is in vision actors vision range. Forced reload of vision actors with currently static vision is expensive and this branch makes sure it's not executed if not needed.
        (bind (_x_2 _y_2) (`self.TransformWorldToGridLocation` (`KismetMathLibrary.MakeVector2D` _returnvalue_x _returnvalue_y)))
        (bind _returnvalue (* (- (`local.X0L`) _x_2) (`self.Tilesize`)))
        (bind _returnvalue_2 (* (- (`local.Y0L`) _y_2) (`self.Tilesize`)))
        (if (<= (+ (* _returnvalue _returnvalue) (* _returnvalue_2 _returnvalue_2)) (* _visionrange _visionrange))
          ;[0.4805 0 0.825] Reload vision
          (`/Game/ClassicRTSFOW/Blueprints/BP_FOW_VisionComponent.ForceReload` (`local.CurrentComponent`) (`|EnumEquality` (`/Game/ClassicRTSFOW/Blueprints/BP_FOW_VisionComponent.StaticVision` (`local.CurrentComponent`)) "NewEnumerator0")))))))

(fn `CreateGrid`
  (params (WorldOrigin :type "Vector2D Structure") (Gridsize :type "Float (double-precision)") (Tilesize :type "Float (double-precision)") (Viewrange :type "Vector2D Structure"))
  (locals (GridsizeL :type "Float (double-precision)"))
  (set `self.WorldOrigin` WorldOrigin)
  (set `local.GridsizeL` Gridsize)
  (set `self.Tilesize` Tilesize)
  (set `self.Viewrange` Viewrange)
  ;[0.2236 0.505 0.07345] Save the size of the squared grid for faster access while transforming from 2D grid index into 1D grid index and vice versa
  (bind _output_get (set `self.Size` (`KismetMathLibrary.FTrunc` (/ (`local.GridsizeL`) (`self.Tilesize`)))))
  ;[0.0412 0.655 0.4066] Create one array element for each tile of the grid and the heightmap
  (for _ (range (+ (* _output_get _output_get) 1))
    (`KismetArrayLibrary.Array_Add` (`self.Grid`) (make `/Game/ClassicRTSFOW/Blueprints/Structs/BP_Tile` true 0.0 (`|MakeArray`)))
    (`KismetArrayLibrary.Array_Add` (`self.Heightmap`))))

(fn `CreateHeightmap`
  (params (WorldTiles :type "Array of /Game/ClassicRTSFOW/Blueprints/BP_HeightmapTile Object Reference"))
  (locals (XL :type Integer) (YL :type Integer) (HeightL :type Integer))
  ;[0.54 0.04036 0] Check if CreateGrid has already been called
  (if (> (`KismetArrayLibrary.Array_Length` (`self.Heightmap`)) 0)
    ;[0.0412 0.655 0.4066] Iterate over all HeightmapTiles
    (for _array_element WorldTiles
      (`|ExecutionSequence`
        (:`then_0`
          (set `local.HeightL` (`/Game/ClassicRTSFOW/Blueprints/BP_HeightmapTile.Height` _array_element))
          (bind _cube (`/Game/ClassicRTSFOW/Blueprints/BP_HeightmapTile.Cube` _array_element))
          (bind (_returnvalue_x _returnvalue_y) (`KismetMathLibrary.BreakVector` (`SceneComponent.K2_GetComponentLocation` _cube)))
          ;[1 0.8709 0] Find out how many and which tiles are covered by the current HeightmapTile. This is a little complicated due to the fact that the location of the HeightmapTile is between 2 tiles if the HeightmapTile covers an even number of tiles in one direction and in the center of one tile when it covers an odd number of tiles
          (bind (_x _y) (`self.TransformWorldToGridLocation` (`KismetMathLibrary.MakeVector2D` _returnvalue_x _returnvalue_y)))
          (set `local.XL` _x)
          (set `local.YL` _y)
          (bind (_returnvalue_x_2 _returnvalue_y_2) (`KismetMathLibrary.BreakVector` (`SceneComponent.K2_GetComponentScale` _cube)))
          (bind _returnvalue (`KismetMathLibrary.FTrunc` _returnvalue_x_2))
          (bind _returnvalue_2 (/ _returnvalue 2))
          (for _index (range (* _returnvalue_2 -1) (+ (select `bool` (== (mod _returnvalue 2) 0) :`false` _returnvalue_2 :`true` (- _returnvalue_2 1)) 1))
            (bind _returnvalue_3 (`KismetMathLibrary.FTrunc` _returnvalue_y_2))
            (bind _returnvalue_4 (/ _returnvalue_3 2))
            (for _index_2 (range (* _returnvalue_4 -1) (+ (select `bool` (== (mod _returnvalue_3 2) 0) :`false` _returnvalue_4 :`true` (- _returnvalue_4 1)) 1))
              (bind _index_3 (`self.Get1DGridIndex` (+ _index (`local.XL`)) (+ _index_2 (`local.YL`))))
              ;[0.54 0.04036 0] Is the current height value bigger than the one the grid already has at that location
              (if (< (`KismetArrayLibrary.Array_Get` (`self.Heightmap`) _index_3) (`local.HeightL`))
                ;[0.4805 0 0.825] Set the new height value
                (`KismetArrayLibrary.Array_Set` (`self.Heightmap`) _index_3 (`local.HeightL`))))))
        (:`then_1`
          (`Actor.K2_DestroyActor` _array_element))))))

(fn `Discover`
  (params (Location :type "Vector2D Structure") (Time :type "Float (double-precision)") (UnitHeight :type Integer) (Static :type "/Game/ClassicRTSFOW/Blueprints/Enums/BP_Static Enum") (Component :type "/Game/ClassicRTSFOW/Blueprints/BP_FOW_VisionComponent Object Reference") (LineOfSight :type Boolean) (VisibleArea :type "/Game/ClassicRTSFOW/Blueprints/Structs/BP_VisibleArea Structure (by ref)"))
  (locals (XL :type Integer :default 0) (YL :type Integer :default 0) (CurrentHeightL :type Integer) (TimeL :type "Float (double-precision)") (CurrentIndexL :type Integer) (VisibleAreaL :type "/Game/ClassicRTSFOW/Blueprints/Structs/BP_VisibleArea Structure" :default (struct)) (UnitHeightL :type Integer) (StaticL :type "/Game/ClassicRTSFOW/Blueprints/Enums/BP_Static Enum") (ListL :type "Array of /Game/ClassicRTSFOW/Blueprints/BP_FOW_VisionComponent Object Reference") (ComponentL :type "/Game/ClassicRTSFOW/Blueprints/BP_FOW_VisionComponent Object Reference") (NotLineOfSightL :type Boolean))
  (bind (_item_discovered _item_fadetime _item_visiblebystatic) (break `/Game/ClassicRTSFOW/Blueprints/Structs/BP_Tile` (`KismetArrayLibrary.Array_Get` (`self.Grid`) (`local.CurrentIndexL`))))
  (bind (_item_discovered_2 _item_fadetime_2 _item_visiblebystatic_2) (break `/Game/ClassicRTSFOW/Blueprints/Structs/BP_Tile` (`KismetArrayLibrary.Array_Get` (`self.Grid`) (`local.CurrentIndexL`))))
  (set `local.TimeL` Time)
  (set `local.UnitHeightL` UnitHeight)
  (set `local.StaticL` Static)
  (set `local.ComponentL` Component)
  (set `local.NotLineOfSightL` (not LineOfSight))
  (`|ExecutionSequence`
    (:`then_0`
      (bind (_x _y) (`self.TransformWorldToGridLocation` Location))
      (set `local.XL` _x)
      (set `local.YL` _y)
      ;[0.2236 0.505 0.07345] Add the height of the unit to the height of the grid the unit is standing on
      (set `local.CurrentHeightL` (+ (`KismetArrayLibrary.Array_Get` (`self.Heightmap`) (`self.Get1DGridIndex` (`local.XL`) (`local.YL`))) (`local.UnitHeightL`))))
    (:`then_1`
      ;[0.0412 0.655 0.4066] Loop along all lines that span the visible area of the actor and stop going along a respective line if the height value of the tile is bigger than the one the unit is standing on  + unit height
      (for _array_element (`.Lines_3_FFB5ECCA439EED13D57CF8B308250D4D` (break `/Game/ClassicRTSFOW/Blueprints/Structs/BP_VisibleArea` VisibleArea))
        (for (_array_element_2 _array_index) (break `/Game/ClassicRTSFOW/Blueprints/Structs/BP_Line` _array_element)
          ;[0.2236 0.505 0.07345] Store the array index of the tile the actor is standing on
          (set `local.CurrentIndexL` (`self.Get1DGridIndex` (+ _array_element_2 (`local.XL`)) (+ (`local.YL`) (`KismetArrayLibrary.Array_Get` (`.Y_8_7D647ED74921C79CB74870927E729AF3` (break `/Game/ClassicRTSFOW/Blueprints/Structs/BP_Line` _array_element)) _array_index))))
          ;[0.54 0.04036 0] Check if the current height >= the height of the heightmap and the current index or if the unit doesn't use line of sight vision
          (if (or (<= (`KismetArrayLibrary.Array_Get` (`self.Heightmap`) (`local.CurrentIndexL`)) (`local.CurrentHeightL`)) (`local.NotLineOfSightL`))
            (switch `/Game/ClassicRTSFOW/Blueprints/Enums/BP_Static` (`local.StaticL`)
              (:`NewEnumerator2`
                ;[0.4805 0 0.825] If the unit uses non-static vision, set the FadeTime of the tile to mark that tile visible until that time. The global time is defined and incremented each Tick within BP_FOW_Actor. Don't touch the VisibleByStatic list in this case.
                (`KismetArrayLibrary.Array_Set` (`self.Grid`) (`local.CurrentIndexL`) (make `/Game/ClassicRTSFOW/Blueprints/Structs/BP_Tile` true (`local.TimeL`) _item_visiblebystatic)))
              (:`NewEnumerator0`
                ;[0.4805 0 0.825] Mark / unmark the tile as visible if the actor switches between static and non-static vision or vice versa by adding / removing this actor from the VisibleByStatic list. Set the tFadeTime like in the case of non-static vision to make sure the tile is visible until FadeTime if the tile is unmarked.
                (bind _output_get (set `local.ListL` _item_visiblebystatic_2))
                (`KismetArrayLibrary.Array_Add` _output_get (`local.ComponentL`))
                (`KismetArrayLibrary.Array_Set` (`self.Grid`) (`local.CurrentIndexL`) (make `/Game/ClassicRTSFOW/Blueprints/Structs/BP_Tile` true (`local.TimeL`) (`local.ListL`)) :!label _label))
              (:`NewEnumerator1`
                (bind _output_get_2 (set `local.ListL` _item_visiblebystatic_2))
                (`KismetArrayLibrary.Array_RemoveItem` _output_get_2 (`local.ComponentL`))
                (goto _label)))
            (else
              (break))))))))

(fn `Get1DGridIndex`
  (params (X :type Integer) (Y :type Integer))
  (returns (Index :type Integer))
  (return (+ (* X (`self.Size`)) Y)))

(fn `Get2DGridIndices`
  (params (Index :type Integer))
  (returns (X :type Integer) (Y :type Integer))
  (bind _size (`self.Size`))
  (return (/ Index _size) (mod Index _size)))

(fn `GetLocationStatus`
  (params (Time :type "Float (double-precision)") (Location :type "Vector2D Structure"))
  (returns (Discovered :type Boolean) (Visible :type Boolean))
  (locals (TimeL :type "Float (double-precision)"))
  (set `local.TimeL` Time)
  (bind (_x _y) (`self.TransformWorldToGridLocation` Location))
  (bind (_discovered _visible) (`self.GetTileStatus` (`local.TimeL`) (`self.Get1DGridIndex` _x _y)))
  (return _discovered _visible))

(fn `GetTileStatus`
  (params (Time :type "Float (double-precision)") (Index :type Integer))
  (returns (Discovered :type Boolean) (Visible :type Boolean))
  (bind (_item_discovered _item_fadetime _item_visiblebystatic) (break `/Game/ClassicRTSFOW/Blueprints/Structs/BP_Tile` (`KismetArrayLibrary.Array_Get` (`self.Grid`) Index)))
  (return _item_discovered (or (<= Time _item_fadetime) (> (`KismetArrayLibrary.Array_Length` _item_visiblebystatic) 0))))

(fn `LoadGrid`
  (params (Location :type "Vector2D Structure"))
  (locals (X :type Integer) (Y :type Integer))
  (bind _viewrange_x (`KismetMathLibrary.BreakVector2D` (`self.Viewrange`)))
  (bind (_viewrange_x_2 _viewrange_y) (`KismetMathLibrary.BreakVector2D` (`self.Viewrange`)))
  (bind _returnvalue (`KismetMathLibrary.FTrunc` (/ (/ _viewrange_y (`self.Tilesize`)) 2.0)))
  (bind _returnvalue_2 (`KismetMathLibrary.FTrunc` (/ (/ _viewrange_x (`self.Tilesize`)) 2.0)))
  (`|ExecutionSequence`
    (:`then_0`
      (`KismetArrayLibrary.Array_Clear` (`self.LowestY`))
      (`KismetArrayLibrary.Array_Clear` (`self.HighestY`)))
    (:`then_1`
      ;[0.2236 0.505 0.07345] Transform the location into WorldGrid space and store the WorldGrid coordinates
      (bind (_x _y) (`self.TransformWorldToGridLocation` Location))
      (set `local.X` _x)
      (set `local.Y` _y))
    (:`then_2`
      ;[0.4805 0 0.825] Store indices for the beginning and the ending for each row of the loaded grid. This way the frequent cost of moving the loaded grid is small and it can easily and readable be iterated over the rows.
      (for _index (range (- (`local.X`) _returnvalue_2) (+ (+ _returnvalue_2 (`local.X`)) 1))
        (`KismetArrayLibrary.Array_Add` (`self.LowestY`) (`self.Get1DGridIndex` _index (- (`local.Y`) _returnvalue)))
        (`KismetArrayLibrary.Array_Add` (`self.HighestY`) (`self.Get1DGridIndex` _index (+ _returnvalue (`local.Y`))))))))

(fn `MoveX`
  (params (NTiles :type Integer))
  (locals (BackwardsL :type Boolean) (RowLength :type Integer) (NTilesL :type Integer))
  (bind _highesty (`self.HighestY`))
  (bind _highesty_2 (`self.HighestY`))
  (bind _lowesty (`self.LowestY`))
  (bind _lowesty_2 (`self.LowestY`))
  (set `local.BackwardsL` (< NTiles 0))
  (set `local.NTilesL` (`KismetMathLibrary.Abs_Int` NTiles))
  (set `local.RowLength` (- (`KismetArrayLibrary.Array_Get` (`self.HighestY`) 1) (`KismetArrayLibrary.Array_Get` (`self.HighestY`))))
  (if (`local.BackwardsL`)
    ;[0.4805 0 0.825] Move the indices that point on the sides of the loaded grid in positive x direction
    (for _ (range 1 (+ (`local.NTilesL`) 1))
      (`|ExecutionSequence`
        (:`then_0`
          (`KismetArrayLibrary.Array_Insert` (`self.LowestY`) (- (`KismetArrayLibrary.Array_Get` (`self.LowestY`)) (`local.RowLength`)))
          (`KismetArrayLibrary.Array_Remove` _lowesty (`KismetArrayLibrary.Array_LastIndex` _lowesty)))
        (:`then_1`
          (`KismetArrayLibrary.Array_Insert` (`self.HighestY`) (- (`KismetArrayLibrary.Array_Get` (`self.HighestY`)) (`local.RowLength`)))
          (`KismetArrayLibrary.Array_Remove` _highesty (`KismetArrayLibrary.Array_LastIndex` _highesty)))))
    (else
      ;[0.4805 0 0.825] Move the indices that point on the sides of the loaded grid in negative x direction
      (for _ (range 1 (+ (`local.NTilesL`) 1))
        (`|ExecutionSequence`
          (:`then_0`
            (`KismetArrayLibrary.Array_Add` (`self.LowestY`) (+ (`KismetArrayLibrary.Array_Get` _lowesty_2 (`KismetArrayLibrary.Array_LastIndex` _lowesty_2)) (`local.RowLength`)))
            (`KismetArrayLibrary.Array_Remove` (`self.LowestY`)))
          (:`then_1`
            (`KismetArrayLibrary.Array_Add` (`self.HighestY`) (+ (`KismetArrayLibrary.Array_Get` _highesty_2 (`KismetArrayLibrary.Array_LastIndex` _highesty_2)) (`local.RowLength`)))
            (`KismetArrayLibrary.Array_Remove` (`self.HighestY`))))))))

(fn `MoveY`
  (params (Backwards :type Boolean) (NTiles :type Integer))
  (locals (BackwardsL :type Boolean) (NTilesL :type Integer))
  (set `local.BackwardsL` Backwards)
  (set `local.NTilesL` NTiles)
  (`|ExecutionSequence`
    (:`then_0`
      ;[0.4805 0 0.825] Move the indices that point on the sides of the loaded grid in positive y direction
      (for (_array_element _array_index) (`self.LowestY`)
        (`KismetArrayLibrary.Array_Set` (`self.LowestY`) _array_index (+ _array_element (`local.NTilesL`)))))
    (:`then_1`
      ;[0.4805 0 0.825] Move the indices that point on the sides of the loaded grid in negative y direction
      (for (_array_element_2 _array_index_2) (`self.HighestY`)
        (`KismetArrayLibrary.Array_Set` (`self.HighestY`) _array_index_2 (+ _array_element_2 (`local.NTilesL`)))))))

(fn `SetMaxVisionRange`
  (params (MaxVisionRange :type "Float (double-precision)"))
  (set `self.MaxVisionRange` MaxVisionRange))

(fn `TransformGridToWorldLocation`
  (params (X :type Integer) (Y :type Integer))
  (returns (ReturnValue :type "Vector2D Structure"))
  (bind _tilesize (`self.Tilesize`))
  (bind (_worldorigin_x _worldorigin_y) (`KismetMathLibrary.BreakVector2D` (`self.WorldOrigin`)))
  (bind _returnvalue (* (`self.Tilesize`) 0.5))
  ;[1 0.8709 0] return the center of the tile in world space
  (return (`KismetMathLibrary.MakeVector2D` (+ (+ (* X _tilesize) _worldorigin_x) _returnvalue) (+ _returnvalue (+ _worldorigin_y (* Y _tilesize))))))

(fn `TransformWorldToGridLocation`
  (params (Location :type "Vector2D Structure"))
  (returns (X :type Integer) (Y :type Integer))
  (bind (_returnvalue_x _returnvalue_y) (`KismetMathLibrary.BreakVector2D` (- Location (`self.WorldOrigin`))))
  (return (`KismetMathLibrary.FTrunc` (/ _returnvalue_x (`self.Tilesize`))) (`KismetMathLibrary.FTrunc` (/ _returnvalue_y (`self.Tilesize`)))))