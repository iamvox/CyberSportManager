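; Actor component that gives its owner team-based vision in an RTS fog-of-war system run by BP_FOW_Actor.
; Moving owners register as frequently updated vision actors, while static ones activate their visible tiles once through Discover.
; Depending on StaticVision, it starts static, never becomes static, or turns static after idling for a set time and reverts on movement.
; ForceReload and SetVisionRange cycle static state to refresh tiles.
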(event `self.ReceiveBeginPlay`
  (`|ExecutionSequence`
    (:`then_0`
      ;[0.2236 0.505 0.07345] Store reference to FOW_Actor for quick access on it
      (bind _outactors (`GameplayStatics.GetAllActorsOfClass` "/Game/ClassicRTSFOW/Blueprints/BP_FOW_Actor.BP_FOW_Actor_C"))
      (set `self.FOW_Actor` (`KismetArrayLibrary.Array_Get` _outactors)))
    (:`then_1`
      (switch `/Game/ClassicRTSFOW/Blueprints/Enums/BP_Type` (`self.StaticVision`)
        (:`NewEnumerator0`
          ;[0.2236 0.505 0.07345] EventTick needs only to be enabled when this actors vision needs to be frequently updated
          (`self.SetComponentTickEnabled` false)
          ;[0 0.009654 1] Make sure BP_FOW_Actor knows what team it is
          (`KismetSystemLibrary.Delay` 0.05)
          ;[0.4805 0 0.825] Activate the tiles visible to this actor.
          (set `self.IsStatic` true)
          (`/Engine/EditorBlueprintResources/StandardMacros.IsValid` (`/Game/ClassicRTSFOW/Blueprints/BP_FOW_Actor.Grid` (`self.FOW_Actor`))
            (:`Is Valid`
              (`/Game/ClassicRTSFOW/Blueprints/BP_FOW_Actor.Discover` (`self.FOW_Actor`) self "NewEnumerator0"))))
        (:`NewEnumerator2`
          (set `self.StaticTimeFrame` 1.0)
          (`self.SetComponentTickEnabled` true :!label _label)
          (`KismetSystemLibrary.Delay` 0.05 :!label _label_2)
          ;[0.4805 0 0.825] Add this actor to VisionActors if its visibility does currently need to be frequently updated.
          (`/Game/ClassicRTSFOW/Blueprints/BP_FOW_Actor.AddVisionActor` (`self.FOW_Actor`) (`self.GetOwner`) (`self.Team`) true))
        (:`NewEnumerator3`
          (set `self.StaticTimeFrame` 2.0)
          (goto _label))
        (:`NewEnumerator4`
          (set `self.StaticTimeFrame` 5.0)
          (goto _label))
        (:`NewEnumerator1`
          (`self.SetComponentTickEnabled` false)
          (goto _label_2))))))

(event `self.ReceiveEndPlay`
  (params (EndPlayReason :type "EEndPlayReason Enum" :default "Destroyed"))
  (if (`self.IsStatic`)
    ;[0.4805 0 0.825] Deactivate the tiles currently visible to this actor
    (`/Game/ClassicRTSFOW/Blueprints/BP_FOW_Actor.Discover` (`self.FOW_Actor`) self "NewEnumerator1")
    (else
      ;[0.4805 0 0.825] Remove this actor from the array of actors whose vision is frequently uploaded
      (`/Game/ClassicRTSFOW/Blueprints/BP_FOW_Actor.RemoveVisionActor` (`self.FOW_Actor`) (`self.GetOwner`)))))

(event `ForceReload`
  (params (StayStatic :type Boolean))
  ;[1 1 1] This event is called when a heightmap tile within vision range of this actor is changed
  (if StayStatic
    (`|ExecutionSequence`
      (:`then_0`
        ;[0.4805 0 0.825] Activate / deactivate all tiles visible to this actor if the static status of this actor is changing
        (if (`self.IsStatic`) :!label _label_3
          (`self.DeactivateStatic`)))
      (:`then_1`
        (if (`self.IsStatic`) :!label _label_4
          _
          (elif (>= (`self.StaticTime`) (`self.StaticTimeFrame`))
            (`self.ActivateStatic`)))))
    (else
      ;[1 0.8709 0] Count the time since this actor moved the last time.
      (set `self.StaticTime` 0.0 :!label _label_5)
      (`|ExecutionSequence`
        (:`then_0`
          (goto _label_3))
        (:`then_1`
          (set `self.LastLocation` (`self.GetActorLocation`)))))))

(event `DeactivateStatic`
  (set `self.IsStatic` false)
  ;[0.4805 0 0.825] Activate / Deactivate all tiles currently visible to this actor
  (`/Game/ClassicRTSFOW/Blueprints/BP_FOW_Actor.Discover` (`self.FOW_Actor`) self "NewEnumerator1")
  ;[0.4805 0 0.825] Add / remove this actor from the array of actors whose vision is frequently uploaded
  (`/Game/ClassicRTSFOW/Blueprints/BP_FOW_Actor.AddVisionActor` (`self.FOW_Actor`) (`self.GetOwner`) (`self.Team`) false))

(event `self.ReceiveTick`
  (params (DeltaSeconds :type "Float (single-precision)"))
  ;[1 0.8709 0] Count the time since this actor moved the last time.
  (set `self.StaticTime` (+ DeltaSeconds (`self.StaticTime`)))
  (if (!= (`self.LastLocation`) (`self.GetActorLocation`))
    (goto _label_5)
    (else
      (goto _label_4))))

(event `ActivateStatic`
  (set `self.IsStatic` true)
  ;[0.4805 0 0.825] Activate / Deactivate all tiles currently visible to this actor
  (`/Game/ClassicRTSFOW/Blueprints/BP_FOW_Actor.Discover` (`self.FOW_Actor`) self "NewEnumerator0")
  ;[0.4805 0 0.825] Add / remove this actor from the array of actors whose vision is frequently uploaded
  (`KismetArrayLibrary.Array_AddUnique` (`/Game/ClassicRTSFOW/Blueprints/BP_FOW_Actor.VisionActorsToRemove` (`self.FOW_Actor`)) (`self.GetOwner`)))

(fn `GetStatic`
  (returns (IsStatic :type Boolean))
  (return (`self.IsStatic`)))

(fn `SetVisionRange`
  (params (NewVisionRange :type "Float (double-precision)"))
  (if (`self.IsStatic`)
    ;[0.4805 0 0.825] This order is needed to make sure no tile holds duplicate entries of this actor and all tiles within the new vision range are activated by this actor
    (`self.DeactivateStatic`)
    (set `self.VisionRange` NewVisionRange)
    (`self.ActivateStatic`)
    (else
      (set `self.VisionRange` NewVisionRange))))