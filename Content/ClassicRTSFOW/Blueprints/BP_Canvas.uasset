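; Fog-of-war painter for the classic RTS FOW system that draws grid tile visibility onto a texture through a Canvas.
; Setters store the grid, time, fog color, tile size and the view parameters used to map world positions into texture space.
; Update redraws every loaded tile as a near-zero-length thick line: visible tiles in the default color, discovered-only tiles in FogColor, and unseen tiles not at all.
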(event `SetTextureSize`
  (params (Texturesize :type "Float (double-precision)"))
  ;[0.2236 0.505 0.07345] Store parameters used to transform points in world coordinate space into texture coordinate space
  (set `self.HalfTexturesize` (* Texturesize 0.5)))

(event `SetViewrange`
  (params (Viewrange :type "Vector2D Structure"))
  ;[0.2236 0.505 0.07345] Store parameters used to transform points in world coordinate space into texture coordinate space
  (bind _output_get (set `self.Viewrange` Viewrange))
  (set `self.Gaugesize` (`KismetMathLibrary.FMax` (`KismetMathLibrary.BreakVector2D` _output_get) (`.Y` (`KismetMathLibrary.BreakVector2D` _output_get)))))

(event `SetCenter`
  (params (Center :type "Vector2D Structure"))
  ;[0.2236 0.505 0.07345] Store parameters used to transform points in world coordinate space into texture coordinate space
  (set `self.Center` Center))

(event `SetTilesize`
  (params (Tilesize :type "Float (double-precision)"))
  (set `self.HalfTilesize` (* Tilesize 0.5)))

(event `SetFogColor`
  (params (FogColor :type "LinearColor Structure"))
  (set `self.FogColor` FogColor))

(event `SetGrid`
  (params (Grid :type "/Game/ClassicRTSFOW/Blueprints/BP_WorldGrid Object Reference (by ref)"))
  (set `self.Grid` Grid))

(event `SetTime`
  (params (Time :type "Float (double-precision)"))
  (set `self.Time` Time))

(event `self.ReceiveUpdate`
  (params (Canvas :type "Canvas Object Reference") (Width :type Integer) (Height :type Integer))
  (`/Engine/EditorBlueprintResources/StandardMacros.IsValid` (`self.Grid`)
    (:`Is Valid`
      ;[0.0412 0.655 0.4066] Iterate over each tile of the loaded grid. The texture has to be fully updated to work properly.
      (for _index (range (+ (`KismetArrayLibrary.Array_LastIndex` (`/Game/ClassicRTSFOW/Blueprints/BP_WorldGrid.LowestY` (`self.Grid`))) 1))
        (for _index_2 (range (`KismetArrayLibrary.Array_Get` (`/Game/ClassicRTSFOW/Blueprints/BP_WorldGrid.LowestY` (`self.Grid`)) _index) (+ (`KismetArrayLibrary.Array_Get` (`/Game/ClassicRTSFOW/Blueprints/BP_WorldGrid.HighestY` (`self.Grid`)) _index) 1))
          ;[0.54 0.04036 0] Check if the tile has to be drawn on the texture
          (bind (_discovered _visible) (`/Game/ClassicRTSFOW/Blueprints/BP_WorldGrid.GetTileStatus` (`self.Grid`) (`self.Time`) _index_2))
          (set `self.Discovered` _discovered)
          (set `self.Visible` _visible)
          (if (or (`self.Visible`) (`self.Discovered`))
            (bind (_x _y) (`/Game/ClassicRTSFOW/Blueprints/BP_WorldGrid.Get2DGridIndices` (`self.Grid`) _index_2))
            ;[1 0.8709 0] Transform the tile's location to the right coordinates
            (bind _returnvalue (`/Game/ClassicRTSFOW/Blueprints/BP_WorldGrid.TransformGridToWorldLocation` (`self.Grid`) _x _y))
            (bind _returnvalue_2 (`self.TransformInTextureCoordinateSpace` _returnvalue))
            ;[0.4805 0 0.825] Draw the tile on the texture
            (if (`self.Visible`)
              (`Canvas.K2_DrawLine` Canvas (`KismetMathLibrary.MakeVector2D` (`KismetMathLibrary.BreakVector2D` _returnvalue_2) (`.Y` (`KismetMathLibrary.BreakVector2D` _returnvalue_2))) (`KismetMathLibrary.MakeVector2D` (+ (`KismetMathLibrary.BreakVector2D` _returnvalue_2) 0.01) (`.Y` (`KismetMathLibrary.BreakVector2D` _returnvalue_2))) (`self.HalfTilesize`) (struct :`R` 1.0 :`G` 1.0 :`B` 1.0 :`A` 1.0))
              (elif (`self.Discovered`)
                (`Canvas.K2_DrawLine` Canvas (`KismetMathLibrary.MakeVector2D` (`KismetMathLibrary.BreakVector2D` _returnvalue_2) (`.Y` (`KismetMathLibrary.BreakVector2D` _returnvalue_2))) (`KismetMathLibrary.MakeVector2D` (+ (`KismetMathLibrary.BreakVector2D` _returnvalue_2) 0.01) (`.Y` (`KismetMathLibrary.BreakVector2D` _returnvalue_2))) (`self.HalfTilesize`) (`self.FogColor`))))))))))

(fn `TransformInTextureCoordinateSpace`
  (params (Vector :type "Vector2D Structure"))
  (returns (ReturnValue :type "Vector2D Structure"))
  (return (* (+ (/ (- Vector (`self.Center`)) (`self.GaugeSize`)) 1.0) (`self.HalfTextureSize`))))