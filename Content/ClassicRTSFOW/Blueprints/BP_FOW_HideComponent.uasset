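; Fog-of-war component that lets its owning actor be hidden and shown in an RTS.
; On BeginPlay it registers the owner and team with the first BP_FOW_Actor found, and unregisters on EndPlay.
; HideActor and ShowActor toggle root component visibility with propagation to children, tracking current and ever-seen state.
; For meleeCreep owners, Team is copied from the creep only after registration has already sent it.
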(event `self.ReceiveBeginPlay`
  (bind _returnvalue (`self.GetOwner`))
  (`|ExecutionSequence`
    (:`then_0`
      ;[0.2236 0.505 0.07345] Store a reference to the FOW_Actor for quick access on EndPlay
      (bind _outactors (`GameplayStatics.GetAllActorsOfClass` "/Game/ClassicRTSFOW/Blueprints/BP_FOW_Actor.BP_FOW_Actor_C"))
      (set `self.FOW_Actor` (`KismetArrayLibrary.Array_Get` _outactors)))
    (:`then_1`
      (`/Game/ClassicRTSFOW/Blueprints/BP_FOW_Actor.AddHideActor` (`self.FOW_Actor`) _returnvalue (stale _output_get)))
    (:`then_2`
      (bind _asmelee_creep (cast `/Game/Actors/CREEPAITESTINGMAP/meleeCreep` _returnvalue))
      (bind _output_get (set `self.Team` (`/Game/Actors/CREEPAITESTINGMAP/meleeCreep.Team` _asmelee_creep))))))

(event `self.ReceiveEndPlay`
  (params (EndPlayReason :type "EEndPlayReason Enum" :default "Destroyed"))
  (`/Game/ClassicRTSFOW/Blueprints/BP_FOW_Actor.RemoveHideActor` (`self.FOW_Actor`) (`self.GetOwner`)))

(fn `GetVisibility`
  (returns (Visible :type Boolean))
  (return (`self.Visible`)))

(fn `HideActor`
  (`SceneComponent.SetVisibility` (`Actor.K2_GetRootComponent` (`self.GetOwner`)) false true)
  (set `self.Visible` false))

(fn `ShowActor`
  (`SceneComponent.SetVisibility` (`Actor.K2_GetRootComponent` (`self.GetOwner`)) true true)
  (set `self.Visible` true)
  (set `self.OnceVisible` true))